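; Playable lobby character with axis-driven movement, mouse look and jump, gated by CanMove, plus a nametag widget.
; MouseY input triggers a camera rotation sync, sending control rotation as integers scaled by 1000 through a multicast event with authority, otherwise a server event.
; The server event only sets the camera rotation, without forwarding to the multicast.
; On BeginPlay the character passes itself to UI_Nametag and hides the widget if locally controlled.
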(event Custom|Multicast%20Sync%20Control%20Rotation
  (params (InInt :type Integer) (InInt2 :type Integer) (InInt3 :type Integer))
  (Transformation|SetWorldRotation (Variables|Default|GetCamera) (Math|Rotator|MakeRotator (/ (Math|Conversions|ToFloat(Integer) InInt) 1e+03) (/ (Math|Conversions|ToFloat(Integer) InInt2) 1e+03) (/ (Math|Conversions|ToFloat(Integer) InInt3) 1e+03)) false false))

(event Custom|UpdateName
  (bind _asui_nametag (Utilities|Casting|CastToUI_Nametag (UserInterface|GetUserWidgetObject (Variables|Default|GetWidget))))
  (Variables|/Game/UI/UI_Nametag.UI_Nametag_C|SetPlayerCharacter _asui_nametag self))

(event Custom|Server%20Sync%20Control%20Rotation
  (params (InInt :type Integer) (InInt2 :type Integer) (InInt3 :type Integer))
  (Transformation|SetWorldRotation (Variables|Default|GetCamera) (Math|Rotator|MakeRotator (/ (Math|Conversions|ToFloat(Integer) InInt) 1e+03) (/ (Math|Conversions|ToFloat(Integer) InInt2) 1e+03) (/ (Math|Conversions|ToFloat(Integer) InInt3) 1e+03)) false false))

(event Custom|CharacterPitchRotation
  (bind _returnvalue (Pawn|GetControlRotation :!class /Script/Engine.Pawn))
  (bind _returnvalue_2 (* (.yaw _returnvalue) 1e+03))
  (bind _returnvalue_3 (* (.roll _returnvalue) 1e+03))
  (bind _returnvalue_4 (* (.pitch _returnvalue) 1e+03))
  (bind _returnvalue_5 (Math|Float|Floor _returnvalue_2))
  (bind _returnvalue_6 (Math|Float|Floor _returnvalue_3))
  (bind _returnvalue_7 (Math|Float|Floor _returnvalue_4))
  (if (Pawn|IsLocallyControlled)
    (if (Ability|HasAuthority)
      (CallFunction|MulticastSyncControlRotation _returnvalue_6 _returnvalue_7 _returnvalue_5)
      (else
        (CallFunction|ServerSyncControlRotation _returnvalue_6 _returnvalue_7 _returnvalue_5)))))

(event EventBeginPlay
  (CallFunction|UpdateName)
  (if (Pawn|IsLocallyControlled)
    (Rendering|SetVisibility (Variables|Default|GetWidget) false false)))

(event Input|ActionEvents|InputActionJump
  (params (Key :type Key%20Structure :default "None"))
  (:Pressed
    (if (Variables|Default|GetCanMove)
      (Character|Jump)))
  (:Released
    (Character|StopJumping)))

(event Input|AxisEvents|InputAxisMouseX
  (params (AxisValue :type Float%20%28single-precision%29))
  (if (Variables|Default|GetCanMove)
    (Pawn|Input|AddControllerYawInput AxisValue)))

(event Input|AxisEvents|InputAxisMouseY
  (params (AxisValue :type Float%20%28single-precision%29))
  (if (Variables|Default|GetCanMove)
    (Pawn|Input|AddControllerPitchInput AxisValue)
    (CallFunction|CharacterPitchRotation)))

(event Input|AxisEvents|InputAxisForward/Backward
  (params (AxisValue :type Float%20%28single-precision%29))
  (if (Variables|Default|GetCanMove)
    (Pawn|Input|AddMovementInput (Math|Vector|GetForwardVector (Math|Rotator|MakeRotator 0.0 0.0 (.Yaw (Math|Rotator|BreakRotator (Pawn|GetControlRotation :!class /Script/Engine.Pawn))))) AxisValue false)))

(event Input|AxisEvents|InputAxisRight/Left
  (params (AxisValue :type Float%20%28single-precision%29))
  (if (Variables|Default|GetCanMove)
    (Pawn|Input|AddMovementInput (Math|Vector|GetRightVector (Math|Rotator|MakeRotator 0.0 0.0 (.Yaw (Math|Rotator|BreakRotator (Pawn|GetControlRotation :!class /Script/Engine.Pawn))))) AxisValue false)))

(fn ConstructionScript)