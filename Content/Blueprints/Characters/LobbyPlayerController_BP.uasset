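; Player controller for the lobby that reports to LobbyGameMode when the local player has loaded in.
; CLIENT events create and remove the LobbyGUI widget and drive its countdown text, tick sounds and screen fade, using a timeline for fade-out.
; Other events blend the view target or switch between play and UI states by toggling input mode, cursor, LobbyCharacter movement and owner mesh visibility, though both hide and unhide set the GUI Hidden.
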(event Custom|CLIENT_ShowLobbyUI
  ;[1 1 1] Client Networking Methods
  (bind _returnvalue (UserInterface|CreateWidget "/Game/UI/LobbyGUI.LobbyGUI_C" (Game|GetPlayerController 0)))
  (bind _output_get (Variables|Default|SetLobbyGUI _returnvalue))
  (UserInterface|Viewport|AddtoViewport _output_get 0)
  (Variables|/Script/Engine.PlayerController|SetbShowMouseCursor (Game|GetPlayerController 0) true))

(event Custom|CLIENT_RemoveLobbyUI
  ;[1 1 1] Client Networking Methods
  (Widget|RemovefromParent (Variables|Default|GetLobbyGUI))
  (Variables|Default|SetLobbyGUI 0))

(event Custom|CLIENT_FadeOutLobby
  ;[1 1 1] Client Networking Methods
  (bind _fadealpha (Timeline|Timeline_0 PlayFromStart)
    (:Update
      (Default|SetFadeScreenOverlayAlpha (Variables|Default|GetLobbyGUI) _fadealpha))))

(event Custom|CLIENT_FadeInLobbyGUI
  ;[1 1 1] Client Networking Methods
  (Default|SetFadeScreenOverlayAlpha (Variables|Default|GetLobbyGUI) 0.0))

(event Custom|CLIENT_UnHideLobbyUI
  (bind _returnvalue (Game|GetPlayerController 0))
  ;[1 1 1] Client Networking Methods
  (Widget|SetVisibility (Variables|Default|GetLobbyGUI) "Hidden")
  (bind _aslobby_character (Utilities|Casting|CastToLobbyCharacter (Game|GetPlayerCharacter 0)))
  (Variables|/Game/Blueprints/Characters/LobbyCharacter.LobbyCharacter_C|SetCanMove _aslobby_character false)
  (Class|PrimitiveComponent|SetOwnerNoSee (Variables|/Script/Engine.Character|GetMesh _aslobby_character) false)
  (Input|SetInputModeUIOnly _returnvalue (Variables|Default|GetLobbyGUI) "LockOnCapture")
  (Variables|/Script/Engine.PlayerController|SetbShowMouseCursor _returnvalue true))

(event Custom|Client_ShowStartingGame
  ;[1 1 1] Client Networking Methods
  (Default|ShowStartingGameText (Variables|Default|GetLobbyGUI))
  (Audio|PlaySound2D "/Game/Sounds/countDownTick.countDownTick" 0.75 0.9 0.0 0 0))

(event Custom|CLIENT_ChangeStartingInText
  (params (Starting%20In :type Integer))
  ;[1 1 1] Client Networking Methods
  (Default|ChangeStartinginText (Variables|Default|GetLobbyGUI) Starting%20In))

(event Custom|CLIENT_HideLobbyUI
  (bind _returnvalue (Game|GetPlayerController 0))
  ;[1 1 1] Client Networking Methods
  (Widget|SetVisibility (Variables|Default|GetLobbyGUI) "Hidden")
  (bind _aslobby_character (Utilities|Casting|CastToLobbyCharacter (Game|GetPlayerCharacter 0)))
  (Class|PrimitiveComponent|SetOwnerNoSee (Variables|/Script/Engine.Character|GetMesh _aslobby_character) true)
  (Variables|/Game/Blueprints/Characters/LobbyCharacter.LobbyCharacter_C|SetCanMove _aslobby_character true)
  (Input|SetInputModeGameOnly _returnvalue)
  (Variables|/Script/Engine.PlayerController|SetbShowMouseCursor _returnvalue false))

(event Custom|SERVER_FullyLoadedIn
  (params (Controller :type Lobby%20Player%20Controller%20BP%20Object%20Reference))
  ;[1 1 1] Server Networking Methods
  (bind _aslobby_game_mode (Utilities|Casting|CastToLobbyGameMode (Game|GetGameMode)))
  (Default|OnPlayerFullyLoadedin _aslobby_game_mode Controller))

(event Custom|CLIENT_PlayCountdownTick
  ;[1 1 1] Client Networking Methods
  (Audio|PlaySound2D "/Game/Sounds/countDownTick.countDownTick" 1.0 1.0 0.0 0 0))

(event Custom|CLIENT_HideStartingGame
  ;[1 1 1] Client Networking Methods
  (Default|HideStartingGameText (Variables|Default|GetLobbyGUI)))

(event Custom|CLIENT_BlendView
  (params (NewViewTarget :type Actor%20Object%20Reference))
  ;[1 1 1] Client Networking Methods
  (Game|Player|SetViewTargetwithBlend self NewViewTarget 1.0 "VTBlend_Linear" 0.0 false))

(event EventBeginPlay
  (bind _returnvalue (Game|GetPlayerController 0))
  (if (Pawn|IsLocalPlayerController)
    (CallFunction|SERVERFullyLoadedin self)
    (Variables|/Script/Engine.PlayerController|SetbShowMouseCursor _returnvalue false)
    (Input|SetInputModeGameOnly _returnvalue)))

(fn ConstructionScript)