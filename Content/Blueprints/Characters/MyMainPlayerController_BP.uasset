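; Player controller for a multiplayer gun-and-knife shooter, acting as the network hub between characters, MainGameMode and GameUI.
; Attacks go to the server, which asks the client for camera aim, line-traces ignoring shooter and dead players, then passes hits to MainGameMode.
; Weapon switches relay through the server to every connected controller.
; Client events drive HUD, countdowns, killfeed, ragdoll toggling, character permissions and look-at rotation; BeginPlay reports test-map loading to the game mode.
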(event Custom|CLIENT_SpawnStrayBullet
  (params (Target :type Vector%20%28by%20ref%29))
  ;[1 1 1] Client Networking Methods
  (bind _asmy_main_character_bp (Utilities|Casting|CastToMyMainCharacter_BP (Game|GetPlayerCharacter 0)))
  (Game|SpawnActorfromClass "/Game/Blueprints/Bullet.Bullet_C" (Math|Transform|MakeTransform (Transformation|GetWorldLocation (Variables|/Game/Blueprints/Characters/MyMainCharacter_BP.MyMainCharacter_BP_C|GetBulletBox _asmy_main_character_bp)) (Math|Rotator|FindLookatRotation (Transformation|GetWorldLocation (Variables|/Game/Blueprints/Characters/MyMainCharacter_BP.MyMainCharacter_BP_C|GetBulletBox _asmy_main_character_bp)) Target)) "Undefined" 0 0))

(event Custom|CLIENT_ShowGameUI
  ;[1 1 1] Client Networking Methods
  (Viewport|RemoveAllWidgets)
  (bind _returnvalue (UserInterface|CreateWidget "/Game/UI/GameUI.GameUI_C" (Game|GetPlayerController 0)))
  (bind _output_get (Variables|Default|SetGameUI _returnvalue))
  (UserInterface|Viewport|AddtoViewport _output_get 0)
  (Variables|/Script/Engine.PlayerController|SetbShowMouseCursor (Game|GetPlayerController 0) false))

(event Custom|SERVER_UpdateWeaponSwitch
  (params (Knife? :type Boolean) (Character :type My%20Main%20Character%20BP%20Object%20Reference))
  ;[1 1 1] Server Networking Methods
  (bind _astesting_game_state_2 (Utilities|Casting|CastToTestingGameState2 (Game|GetGameState)))
  (bind _returnvalue (Class|TestingGameState2|GetPlayersConnected _astesting_game_state_2))
  (for _array_element _returnvalue
    (bind _asmy_main_player_controller_bp (Utilities|Casting|CastToMyMainPlayerController_BP _array_element))
    (CallFunction|CLIENTSwitchGunorKnife _asmy_main_player_controller_bp Knife? Character)))

(event Custom|CLIENT_SpawnBullet
  (params (Target :type Vector%20%28by%20ref%29))
  ;[1 1 1] Client Networking Methods
  (bind _asmy_main_character_bp (Utilities|Casting|CastToMyMainCharacter_BP (Game|GetPlayerCharacter 0)))
  (Game|SpawnActorfromClass "/Game/Blueprints/Bullet.Bullet_C" (Math|Transform|MakeTransform (Transformation|GetWorldLocation (Variables|/Game/Blueprints/Characters/MyMainCharacter_BP.MyMainCharacter_BP_C|GetBulletBox _asmy_main_character_bp)) (Math|Rotator|FindLookatRotation (Transformation|GetWorldLocation (Variables|/Game/Blueprints/Characters/MyMainCharacter_BP.MyMainCharacter_BP_C|GetBulletBox _asmy_main_character_bp)) Target)) "Undefined" 0 0))

(event Custom|CLIENT_SetScore3
  (params (Name :type String) (Score :type String))
  ;[1 1 1] Client Networking Methods
  (Default|SetScore3 (Variables|Default|GetGameUI) Name Score))

(event Custom|CLIENT_FadeInBlurGameOver
  ;[1 1 1] Client Networking Methods
  (bind _newtrack_0 (Timeline|Timeline_1 PlayFromStart)
    (:Update
      (Class|BackgroundBlur|SetBlurStrength (Variables|/Game/UI/GameUI.GameUI_C|GetGameOverBackgroundBlur (Variables|Default|GetGameUI)) _newtrack_0))))

(event Custom|CLIENT_ShowMenuUI
  ;[1 1 1] Client Networking Methods
  (bind _returnvalue (UserInterface|CreateWidget "/Game/UI/MainMenuGUI.MainMenuGUI_C" (Game|GetPlayerController 0)))
  (UserInterface|Viewport|AddtoViewport _returnvalue 0)
  (Variables|/Script/Engine.PlayerController|SetbShowMouseCursor (Game|GetPlayerController 0) true))

(event Custom|CLIENT_HideScore3
  ;[1 1 1] Client Networking Methods
  (Default|DisableScore3 (Variables|Default|GetGameUI)))

(event Custom|CLIENT_DenyMovement
  ;[1 1 1] Client Networking Methods
  (bind _asmy_main_character_bp (Utilities|Casting|CastToMyMainCharacter_BP (Game|GetPlayerCharacter 0)))
  (Variables|/Game/Blueprints/Characters/MyMainCharacter_BP.MyMainCharacter_BP_C|SetCanMove _asmy_main_character_bp false))

(event Custom|CLIENT_SetScore1
  (params (Name :type String) (Score :type String))
  ;[1 1 1] Client Networking Methods
  (Default|SetScore1 (Variables|Default|GetGameUI) Name Score))

(event Custom|CLIENT_TellAllClientsSwitchWeapon
  (params (SwitchToKnife :type Boolean) (Character :type My%20Main%20Character%20BP%20Object%20Reference))
  (CallFunction|SERVERUpdateWeaponSwitch SwitchToKnife Character))

(event Custom|CLIENT_StartGameCountdown
  (bind _gameui (Variables|Default|GetGameUI))
  ;[1 1 1] Client Networking Methods
  (Widget|SetVisibility (Variables|/Game/UI/GameUI.GameUI_C|GetStartingPanel _gameui) "SelfHitTestInvisible")
  (Widget|SetVisibility (Variables|/Game/UI/GameUI.GameUI_C|GetWaitingPanel _gameui) "Hidden")
  (bind _fadealpha (Timeline|Timeline_2 PlayFromStart)
    (:Update
      (Class|BackgroundBlur|SetBlurStrength (Variables|/Game/UI/GameUI.GameUI_C|GetStartingBackgroundBlur (Variables|Default|GetGameUI)) _fadealpha))))

(event Custom|CLIENT_SetScore2
  (params (Name :type String) (Score :type String))
  ;[1 1 1] Client Networking Methods
  (Default|SetScore2 (Variables|Default|GetGameUI) Name Score))

(event Custom|CLIENT_AddKillFeed
  (params (Killer :type String) (Killed :type String))
  ;[1 1 1] Client Networking Methods
  (bind _returnvalue (UserInterface|CreateWidget "/Game/UI/Killed_Slot.Killed_Slot_C" 0 Killer Killed))
  (Widget|Panel|AddChild (Variables|/Game/UI/Killfeed.Killfeed_C|GetVerticalBox_61 (Variables|/Game/UI/GameUI.GameUI_C|GetKillfeed (Variables|Default|GetGameUI))) _returnvalue))

(event Custom|CLIENT_SetStartingInTextGame
  (params (Starting%20In :type Integer))
  ;[1 1 1] Client Networking Methods
  (Default|ChangeStartinginText (Variables|Default|GetGameUI) Starting%20In)
  (Audio|PlaySound2D "/Game/Sounds/countDownTick.countDownTick" 1.0 1.0 0.0 0 0))

(event Custom|CLIENT_ShowFullGameUI
  (bind _gameui (Variables|Default|GetGameUI))
  ;[1 1 1] Client Networking Methods
  (Widget|SetVisibility (Variables|/Game/UI/GameUI.GameUI_C|GetGamePanel _gameui) "SelfHitTestInvisible")
  (Widget|SetVisibility (Variables|/Game/UI/GameUI.GameUI_C|GetStartingPanel _gameui) "Hidden"))

(event Custom|CLIENT_AllowMovement
  ;[1 1 1] Client Networking Methods
  (bind _asmy_main_character_bp (Utilities|Casting|CastToMyMainCharacter_BP (Game|GetPlayerCharacter 0)))
  (Variables|/Game/Blueprints/Characters/MyMainCharacter_BP.MyMainCharacter_BP_C|SetCanMove _asmy_main_character_bp true))

(event Custom|CLIENT_AddDisconnectToFeed
  (params (Name :type String))
  ;[1 1 1] Client Networking Methods
  (bind _returnvalue (UserInterface|CreateWidget "/Game/UI/Connection_Slot.Connection_Slot_C" 0 Name))
  (Widget|Panel|AddChild (Variables|/Game/UI/Killfeed.Killfeed_C|GetVerticalBox_61 (Variables|/Game/UI/GameUI.GameUI_C|GetKillfeed (Variables|Default|GetGameUI))) _returnvalue))

(event Custom|SERVER_Knife
  (params (NewParam :type My%20Main%20Player%20Controller%20BP%20Object%20Reference))
  ;[1 1 1] Server Networking Methods
  (CallFunction|CLIENTSetAllowKnife NewParam false)
  (CallFunction|CLIENTKnife)
  (Utilities|FlowControl|Delay 0.5)
  (CallFunction|CLIENTSetAllowKnife true))

(event Custom|CLIENT_Knife
  ;[1 1 1] Client Networking Methods
  (bind _asmy_main_character_bp (Utilities|Casting|CastToMyMainCharacter_BP (Game|GetPlayerCharacter 0)))
  (CallFunction|SERVERProcessKnife (Transformation|GetWorldLocation (Variables|/Game/Blueprints/Characters/MyMainCharacter_BP.MyMainCharacter_BP_C|GetCamera _asmy_main_character_bp)) (+ (Transformation|GetWorldLocation (Variables|/Game/Blueprints/Characters/MyMainCharacter_BP.MyMainCharacter_BP_C|GetCamera _asmy_main_character_bp)) (* (Math|Vector|GetForwardVector (Transformation|GetWorldRotation (Variables|/Game/Blueprints/Characters/MyMainCharacter_BP.MyMainCharacter_BP_C|GetCamera _asmy_main_character_bp))) 4.5e+02)) _asmy_main_character_bp))

(event Custom|CLIENT_ShowGameOverUI
  ;[1 1 1] Client Networking Methods
  (Widget|SetVisibility (Variables|/Game/UI/GameUI.GameUI_C|GetGameOverPanel (Variables|Default|GetGameUI)) "SelfHitTestInvisible"))

(event Custom|SERVER_NotifyTestMapLoaded
  (params (NewParam :type My%20Main%20Player%20Controller%20BP%20Object%20Reference))
  ;[1 1 1] Server Networking Methods
  (bind _asmain_game_mode (Utilities|Casting|CastToMainGameMode (Game|GetGameMode)))
  (Default|PlayerFInishedLoadingin _asmain_game_mode NewParam))

(event Custom|CLIENT_SetTimeLeft
  (params (TimeLeft :type Integer))
  ;[1 1 1] Client Networking Methods
  (Default|ChangeTimeText (Variables|Default|GetGameUI) TimeLeft))

(event Custom|CLIENT_SetMouseAction
  (params (CanDoMouseActions? :type Boolean))
  ;[1 1 1] Client Networking Methods
  (bind _asmy_main_character_bp (Utilities|Casting|CastToMyMainCharacter_BP (Game|GetPlayerCharacter 0)))
  (Variables|/Game/Blueprints/Characters/MyMainCharacter_BP.MyMainCharacter_BP_C|SetCanDoMouseActions? _asmy_main_character_bp CanDoMouseActions?))

(event Custom|CLIENT_SetAmmoText
  (params (Ammo :type String))
  ;[1 1 1] Client Networking Methods
  (Rendering|Components|TextRender|SetText (Variables|/Game/UI/GameUI.GameUI_C|GetGunAmmoText (Variables|Default|GetGameUI)) (Utilities|Text|ToText(String) Ammo)))

(event Custom|Knife
  (bind _asmy_main_player_controller_bp (Utilities|Casting|CastToMyMainPlayerController_BP (Game|GetPlayerController 0)))
  (CallFunction|SERVERKnife _asmy_main_player_controller_bp))

(event Custom|CLIENT_SetGameWinner
  (params (NewParam :type String))
  ;[1 1 1] Client Networking Methods
  (Rendering|Components|TextRender|SetText (Variables|/Game/UI/GameUI.GameUI_C|GetPlayerNameText (Variables|Default|GetGameUI)) (Utilities|Text|ToText(String) NewParam)))

(event Custom|CLIENT_RotateAroundPlayer
  (params (RotateTo :type My%20Main%20Character%20BP%20Object%20Reference))
  ;[1 1 1] Client Networking Methods
  (Variables|Default|SetRotateAround RotateTo)
  (Variables|Default|SetCanRotate true))

(event Custom|CLIENT_SetScoreText
  (params (Score :type Integer))
  ;[1 1 1] Client Networking Methods
  (Rendering|Components|TextRender|SetText (Variables|/Game/UI/GameUI.GameUI_C|GetScoreText (Variables|Default|GetGameUI)) (Utilities|Text|ToText(Integer) Score)))

(event Custom|CLIENT_ReshowGameUI
  ;[1 1 1] Client Networking Methods
  (Widget|SetVisibility (Variables|/Game/UI/GameUI.GameUI_C|GetGamePanel (Variables|Default|GetGameUI)) "SelfHitTestInvisible"))

(event Custom|CLIENT_EnableGunMesh
  ;[1 1 1] Client Networking Methods
  (bind _asmy_main_character_bp (Utilities|Casting|CastToMyMainCharacter_BP (Game|GetPlayerCharacter 0)))
  (Development|SetHiddeninGame (Variables|/Game/Blueprints/Characters/MyMainCharacter_BP.MyMainCharacter_BP_C|GetCoolLowPolyGun _asmy_main_character_bp) false false))

(event Custom|CLIENT_HideDeathUI
  ;[1 1 1] Client Networking Methods
  (Widget|SetVisibility (Variables|/Game/UI/GameUI.GameUI_C|GetDeadPanel (Variables|Default|GetGameUI)) "Hidden"))

(event Custom|CLIENT_StopRotate
  ;[1 1 1] Client Networking Methods
  (Variables|Default|SetRotateAround 0)
  (Variables|Default|SetCanRotate false))

(event Custom|CLIENT_SetRespawningInText
  (params (Time :type String))
  ;[1 1 1] Client Networking Methods
  (Default|ChangeRespawningText (Variables|Default|GetGameUI) Time)
  (Audio|PlaySound2D "/Game/Sounds/countDownTick.countDownTick" 1.0 1.0 0.0 0 0))

(event Custom|CLIENT_SetReturningToLobbyText
  (params (Time :type String))
  ;[1 1 1] Client Networking Methods
  (Default|ChangeReturningtoLobbyText (Variables|Default|GetGameUI) Time))

(event Custom|MULTICAST_GunShot
  (params (Location :type Vector))
  ;[1 1 1] Multicast Networking Methods
  (Audio|PlaySoundatLocation "/Game/Sounds/FireSound_2.FireSound_2" Location "0, 0, 0" 1.0 1.0 0.0 0 0 0))

(event Custom|CLIENT_HideGameUI
  ;[1 1 1] Client Networking Methods
  (Widget|SetVisibility (Variables|/Game/UI/GameUI.GameUI_C|GetGamePanel (Variables|Default|GetGameUI)) "Hidden"))

(event Custom|CLIENT_Disconnect
  ;[1 1 1] Client Networking Methods
  (|Logout (Game|GetPlayerController 0)
    (:OnSuccess
      (Game|OpenLevel(byName) "MainMenu"))
    (:OnFailure
      (Development|PrintString "Failed to Leave session."))))

(event Custom|Shoot
  (bind _asmy_main_player_controller_bp (Utilities|Casting|CastToMyMainPlayerController_BP (Game|GetPlayerController 0)))
  (CallFunction|SERVERShoot _asmy_main_player_controller_bp))

(event Custom|CLIENT_SetDeathByText
  (params (Killed%20By :type String))
  ;[1 1 1] Client Networking Methods
  (Default|ChangeKilledbyText (Variables|Default|GetGameUI) Killed%20By))

(event Custom|CLIENT_PreProcessShot
  ;[1 1 1] Client Networking Methods
  (bind _asmy_main_character_bp (Utilities|Casting|CastToMyMainCharacter_BP (Game|GetPlayerCharacter 0)))
  (CallFunction|SERVERProcessShot (Transformation|GetWorldLocation (Variables|/Game/Blueprints/Characters/MyMainCharacter_BP.MyMainCharacter_BP_C|GetCamera _asmy_main_character_bp)) (+ (Transformation|GetWorldLocation (Variables|/Game/Blueprints/Characters/MyMainCharacter_BP.MyMainCharacter_BP_C|GetCamera _asmy_main_character_bp)) (* (Math|Vector|GetForwardVector (Transformation|GetWorldRotation (Variables|/Game/Blueprints/Characters/MyMainCharacter_BP.MyMainCharacter_BP_C|GetCamera _asmy_main_character_bp))) 1e+04)) _asmy_main_character_bp))

(event Custom|CLIENT_SetDistanceText
  (params (Distance :type String))
  ;[1 1 1] Client Networking Methods
  (Default|ChangeDistanceText (Variables|Default|GetGameUI) Distance))

(event Custom|CLIENT_ShowDeathUI
  ;[1 1 1] Client Networking Methods
  (Widget|SetVisibility (Variables|/Game/UI/GameUI.GameUI_C|GetDeadPanel (Variables|Default|GetGameUI)) "SelfHitTestInvisible"))

(event Custom|SERVER_Shoot
  (params (NewParam :type My%20Main%20Player%20Controller%20BP%20Object%20Reference))
  ;[1 1 1] Server Networking Methods
  (CallFunction|CLIENTSetAllowShoot NewParam false)
  (CallFunction|CLIENTPreProcessShot NewParam)
  (CallFunction|MULTICASTGunShot (Transformation|GetActorLocation (Pawn|GetControlledPawn NewParam)))
  (bind _asmy_main_character_bp (Utilities|Casting|CastToMyMainCharacter_BP (Pawn|GetControlledPawn NewParam)))
  (bind _output_get (Variables|/Game/Blueprints/Characters/MyMainCharacter_BP.MyMainCharacter_BP_C|SetAmmoCount _asmy_main_character_bp (- (Variables|/Game/Blueprints/Characters/MyMainCharacter_BP.MyMainCharacter_BP_C|GetAmmoCount _asmy_main_character_bp) 1)))
  (if (> _output_get 0)
    (CallFunction|CLIENTSetAllowShoot true)
    (CallFunction|CLIENTSetAmmoText NewParam (Utilities|String|ToString(Integer) _output_get))
    (else
      (CallFunction|CLIENTSetAmmoText NewParam "0")
      (CallFunction|CLIENTSetAllowShoot false))))

(event Custom|SERVER_ProcessShot
  (params (Start :type Vector) (End :type Vector) (Shooter :type My%20Main%20Character%20BP%20Object%20Reference))
  ;[1 1 1] Server Networking Methods
  (bind _astesting_game_state_2 (Utilities|Casting|CastToTestingGameState2 (Game|GetGameState)))
  (bind _returnvalue (Class|TestingGameState2|GetPlayersDead _astesting_game_state_2))
  (for _array_element _returnvalue
    (bind _asmy_main_character_bp (Utilities|Casting|CastToMyMainCharacter_BP (Pawn|GetControlledPawn _array_element)))
    (Utilities|Array|Add (Variables|Default|GetNewVar_0) _asmy_main_character_bp))
  (Utilities|Array|Add (Variables|Default|GetNewVar_0) Shooter)
  (bind (_outhit _returnvalue_2) (Collision|LineTraceForObjects Start End (Utilities|Array|MakeArray "ObjectTypeQuery1") false (Variables|Default|GetNewVar_0) "None"))
  (Utilities|Array|Clear (Variables|Default|GetNewVar_0))
  (if _returnvalue_2
    (bind _asmain_game_mode (Utilities|Casting|CastToMainGameMode (Game|GetGameMode)))
    (Default|ProcessHitResult _asmain_game_mode _outhit Shooter)
    (else
      (bind _asmy_main_player_controller_bp (Utilities|Casting|CastToMyMainPlayerController_BP (Pawn|GetController Shooter)))
      (CallFunction|CLIENTSpawnStrayBullet _asmy_main_player_controller_bp End))))

(event Custom|CLIENT_SetAllowShoot
  (params (AllowShoot? :type Boolean))
  ;[1 1 1] Client Networking Methods
  (bind _asmy_main_character_bp (Utilities|Casting|CastToMyMainCharacter_BP (Game|GetPlayerCharacter 0)))
  (Variables|/Game/Blueprints/Characters/MyMainCharacter_BP.MyMainCharacter_BP_C|SetAllowedToShoot? _asmy_main_character_bp AllowShoot?))

(event Custom|CLIENT_SwitchGunOrKnife
  (params (SwitchToKnife :type Boolean) (Character :type My%20Main%20Character%20BP%20Object%20Reference))
  (bind _gun___owner_no_see (Variables|/Game/Blueprints/Characters/MyMainCharacter_BP.MyMainCharacter_BP_C|GetGun%20-%20Owner%20No%20See Character))
  (bind _knife (Variables|/Game/Blueprints/Characters/MyMainCharacter_BP.MyMainCharacter_BP_C|GetKnife Character))
  (bind _knife___owner_no_see (Variables|/Game/Blueprints/Characters/MyMainCharacter_BP.MyMainCharacter_BP_C|GetKnife%20-%20Owner%20No%20See Character))
  (bind _coollowpolygun (Variables|/Game/Blueprints/Characters/MyMainCharacter_BP.MyMainCharacter_BP_C|GetCoolLowPolyGun Character))
  (if SwitchToKnife
    (Rendering|SetVisibility _knife true false)
    (Rendering|SetVisibility _knife___owner_no_see true false)
    (Rendering|SetVisibility _coollowpolygun false false)
    (Rendering|SetVisibility _gun___owner_no_see false false)
    (else
      (Rendering|SetVisibility _knife false false)
      (Rendering|SetVisibility _knife___owner_no_see false false)
      (Rendering|SetVisibility _coollowpolygun true false)
      (Rendering|SetVisibility _gun___owner_no_see true false))))

(event Custom|CLIENT_PlayerChangeVisiblity
  (params (Make%20Visible? :type Boolean) (Character :type My%20Main%20Character%20BP%20Object%20Reference))
  (bind _capsulecomponent (Variables|/Script/Engine.Character|GetCapsuleComponent Character))
  (bind _mesh (Variables|/Script/Engine.Character|GetMesh Character))
  (bind _mesh_2 (Variables|/Script/Engine.Character|GetMesh Character))
  (if Make%20Visible?
    (Physics|SetSimulatePhysics _mesh_2 false)
    (Transformation|SetRelativeLocationAndRotation _mesh_2 "0,0.000000,-90.000000" "0.000000,-90.000000, 0" false false)
    (Transformation|AttachComponentToComponent _mesh_2 (Variables|/Script/Engine.Actor|GetRootComponent Character) "None" "KeepRelative" "KeepRelative" "KeepRelative" true)
    (Collision|SetCollisionProfileName _mesh_2 "BlockAll" true :!class /Script/Engine.PrimitiveComponent)
    (Collision|SetCollisionEnabled _capsulecomponent "QueryAndPhysics")
    (else
      (Physics|SetSimulatePhysics _mesh true)
      (Collision|SetCollisionProfileName _mesh "Ragdoll" true :!class /Script/Engine.PrimitiveComponent)
      (Collision|SetCollisionEnabled _capsulecomponent "NoCollision"))))

(event Custom|CLIENT_SetAllowKnife
  (params (AllowKnife? :type Boolean))
  ;[1 1 1] Client Networking Methods
  (bind _asmy_main_character_bp (Utilities|Casting|CastToMyMainCharacter_BP (Game|GetPlayerCharacter 0)))
  (Variables|/Game/Blueprints/Characters/MyMainCharacter_BP.MyMainCharacter_BP_C|SetAllowedToKnife? _asmy_main_character_bp AllowKnife?))

(event Custom|SERVER_ProcessKnife
  (params (Start :type Vector) (End :type Vector) (Shooter :type My%20Main%20Character%20BP%20Object%20Reference))
  ;[1 1 1] Server Networking Methods
  (bind _astesting_game_state_2 (Utilities|Casting|CastToTestingGameState2 (Game|GetGameState)))
  (bind _returnvalue (Class|TestingGameState2|GetPlayersDead _astesting_game_state_2))
  (for _array_element _returnvalue
    (bind _asmy_main_character_bp (Utilities|Casting|CastToMyMainCharacter_BP (Pawn|GetControlledPawn _array_element)))
    (Utilities|Array|Add (Variables|Default|GetNewVar_0) _asmy_main_character_bp))
  (Utilities|Array|Add (Variables|Default|GetNewVar_0) Shooter)
  (bind (_outhit _returnvalue_2) (Collision|LineTraceForObjects Start End (Utilities|Array|MakeArray "ObjectTypeQuery1") false (Variables|Default|GetNewVar_0) "None"))
  (Utilities|Array|Clear (Variables|Default|GetNewVar_0))
  (if _returnvalue_2
    (bind _asmain_game_mode (Utilities|Casting|CastToMainGameMode (Game|GetGameMode)))
    (Default|ProcessHitResult _asmain_game_mode _outhit Shooter)))

(event Custom|CLIENT_SetKnifeDisabled
  (params (KnifeDisabled? :type Boolean))
  ;[1 1 1] Client Networking Methods
  (bind _asmy_main_character_bp (Utilities|Casting|CastToMyMainCharacter_BP (Game|GetPlayerCharacter 0)))
  (Variables|/Game/Blueprints/Characters/MyMainCharacter_BP.MyMainCharacter_BP_C|SetKnifeDisabled? _asmy_main_character_bp KnifeDisabled?))

(event Custom|CLIENT_SetGunActive
  (params (GunActive? :type Boolean))
  ;[1 1 1] Client Networking Methods
  (bind _asmy_main_character_bp (Utilities|Casting|CastToMyMainCharacter_BP (Game|GetPlayerCharacter 0)))
  (Variables|/Game/Blueprints/Characters/MyMainCharacter_BP.MyMainCharacter_BP_C|SetGunActive _asmy_main_character_bp GunActive?))

(event Custom|CLIENT_DisableGunMesh
  ;[1 1 1] Client Networking Methods
  (bind _asmy_main_character_bp (Utilities|Casting|CastToMyMainCharacter_BP (Game|GetPlayerCharacter 0)))
  (Development|SetHiddeninGame (Variables|/Game/Blueprints/Characters/MyMainCharacter_BP.MyMainCharacter_BP_C|GetCoolLowPolyGun _asmy_main_character_bp) true false))

(event Custom|CLIENT_PlayHitMarker
  ;[1 1 1] Client Networking Methods
  (Audio|PlaySound2D "/Game/Sounds/Hit_Marker.Hit_Marker" 1.0 1.0 0.0 0 0))

(event Custom|CLIENT_SetGunDisabled
  (params (GunDisabled? :type Boolean))
  ;[1 1 1] Client Networking Methods
  (bind _asmy_main_character_bp (Utilities|Casting|CastToMyMainCharacter_BP (Game|GetPlayerCharacter 0)))
  (Variables|/Game/Blueprints/Characters/MyMainCharacter_BP.MyMainCharacter_BP_C|SetGunDisabled? _asmy_main_character_bp GunDisabled?))

(event EventTick
  (params (DeltaSeconds :type Float%20%28single-precision%29))
  (if (Variables|Default|GetCanRotate)
    (Pawn|SetControlRotation (Math|Interpolation|RInterpTo (Pawn|GetControlRotation :!class /Script/Engine.Controller) (Math|Rotator|FindLookatRotation (Transformation|GetActorLocation (Game|GetPlayerCharacter 0)) (Transformation|GetActorLocation (Variables|Default|GetRotateAround))) (Utilities|Time|GetWorldDeltaSeconds) 2.0))))

(event EventBeginPlay
  (if (Pawn|IsLocalPlayerController)
    (bind _returnvalue (Game|GetCurrentLevelName true))
    (if (Utilities|Enum|Equal(Enum) _returnvalue "TestingLevel")
      (bind _asmy_main_player_controller_bp (Utilities|Casting|CastToMyMainPlayerController_BP (Game|GetPlayerController 0)))
      (CallFunction|SERVERNotifyTestMapLoaded _asmy_main_player_controller_bp _asmy_main_player_controller_bp)
      (elif (Utilities|Enum|Equal(Enum) _returnvalue "TestLevel2")
        (bind _asmy_main_player_controller_bp_2 (Utilities|Casting|CastToMyMainPlayerController_BP (Game|GetPlayerController 0)))
        (CallFunction|SERVERNotifyTestMapLoaded _asmy_main_player_controller_bp_2 _asmy_main_player_controller_bp_2)))))

(fn ConstructionScript)