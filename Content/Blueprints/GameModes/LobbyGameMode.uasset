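; Lobby game mode that starts the match countdown once at least two players are connected and cancels it when the count drops.
; StartGame, StopGameStart and timer queries are defined outside this graph; events here relay countdown text, final-five-second ticks and fades to each LobbyPlayerController_BP through client calls.
; The final seconds also update the session as joinable and not mid-game, and late joiners receive the running countdown.
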(event Custom|Hide%20Starting%20Game%20Text
  ;[1 1 1] Text Code
  (bind _astesting_game_state (Utilities|Casting|CastToTestingGameState (Game|GetGameState)))
  (bind _returnvalue (Class|TestingGameState|GetPlayersConnected _astesting_game_state))
  (for _array_element _returnvalue
    (bind _aslobby_player_controller_bp (Utilities|Casting|CastToLobbyPlayerController_BP _array_element))
    (Default|ClientHideStartingGame _aslobby_player_controller_bp)))

(event Custom|On%20Player%20Fully%20Loaded%20In
  (params (Controller :type Lobby%20Player%20Controller%20BP%20Object%20Reference))
  (bind _returnvalue (Class|TestingGamemode|IsStarting))
  (if _returnvalue
    (CallFunction|ShowStartingGameTextforPlayer Controller)
    (bind _returnvalue_2 (Class|TestingGamemode|GetTimeTilStart))
    (CallFunction|SetStartingGameTimeforPlayer Controller _returnvalue_2)
    (else
      (CallFunction|CheckifCanStart))))

(event Custom|Show%20Starting%20Game%20Text
  ;[1 1 1] Text Code
  (bind _astesting_game_state (Utilities|Casting|CastToTestingGameState (Game|GetGameState)))
  (bind _returnvalue (Class|TestingGameState|GetPlayersConnected _astesting_game_state))
  (for _array_element _returnvalue
    (bind _aslobby_player_controller_bp (Utilities|Casting|CastToLobbyPlayerController_BP _array_element))
    (Default|ClientShowStartingGame _aslobby_player_controller_bp)))

(event Custom|Check%20If%20Can%20Start
  (bind _astesting_game_state (Utilities|Casting|CastToTestingGameState (Game|GetGameState)))
  (bind _returnvalue (Class|TestingGameState|GetPlayersConnected _astesting_game_state))
  (if (!= (Utilities|Array|Length _returnvalue) 0)
    (if (>= (Utilities|Array|Length _returnvalue) 2)
      (if (not (Variables|Default|GetAllowedToStart))
        (Variables|Default|SetAllowedToStart true)
        (CallFunction|ShowStartingGameText)
        (Class|TestingGamemode|StartGame))
      (else
        (if (Variables|Default|GetAllowedToStart) :!label _label
          (Variables|Default|SetAllowedToStart false)
          (CallFunction|HideStartingGameText)
          (Class|TestingGamemode|StopGameStart))))
    (else
      (goto _label))))

(event Custom|Show%20Starting%20Game%20Text%20For%20Player
  (params (Controller :type Lobby%20Player%20Controller%20BP%20Object%20Reference))
  ;[1 1 1] Text Code
  (Default|ClientShowStartingGame Controller))

(event Custom|Set%20Starting%20Game%20Time%20For%20Player
  (params (Controller :type Lobby%20Player%20Controller%20BP%20Object%20Reference) (Starting%20In :type Integer))
  ;[1 1 1] Text Code
  (Default|CLIENTChangeStartinginText Controller Starting%20In))

(event EventShowLobbyUI
  (params (PlayerController :type Player%20Controller%20Object%20Reference))
  (bind _aslobby_player_controller_bp (Utilities|Casting|CastToLobbyPlayerController_BP PlayerController))
  (Default|CLIENTShowLobbyUI _aslobby_player_controller_bp)
  (CallFunction|CheckifCanStart))

(event EventOnLogout
  (params (ExitingController :type Controller%20Object%20Reference))
  ;[1 1 1] Connection Code
  (Utilities|Casting|CastToMyMainPlayerController_BP ExitingController)
  (CallFunction|CheckifCanStart))

(event EventPostLogin
  (params (NewPlayer :type Player%20Controller%20Object%20Reference))
  ;[1 1 1] Connection Code
)

(event EventChangeLobbyStartingText
  (params (TimeLeftUntilStart :type Integer))
  ;[1 1 1] Text Code
  (bind _astesting_game_state (Utilities|Casting|CastToTestingGameState (Game|GetGameState)))
  (bind _returnvalue (Class|TestingGameState|GetPlayersConnected _astesting_game_state))
  (for _array_element _returnvalue
    (bind _aslobby_player_controller_bp (Utilities|Casting|CastToLobbyPlayerController_BP _array_element))
    (Default|CLIENTChangeStartinginText _aslobby_player_controller_bp TimeLeftUntilStart)
    (bind _returnvalue_2 (Class|TestingGamemode|GetTimeTilStart))
    (if (<= _returnvalue_2 5)
      (Default|CLIENTPlayCountdownTick _aslobby_player_controller_bp)
      (|UpdateSession (Utilities|Array|MakeArray (Class|AdvancedSessionsLibrary|MakeLiteralSessionPropertyBool "Mid-Game" false)) 10 0 false true true true false))))

(event EventFadeIntoGame
  (bind _astesting_game_state (Utilities|Casting|CastToTestingGameState (Game|GetGameState)))
  (bind _returnvalue (Class|TestingGameState|GetPlayersConnected _astesting_game_state))
  (for _array_element _returnvalue
    (bind _aslobby_player_controller_bp (Utilities|Casting|CastToLobbyPlayerController_BP _array_element))
    (Default|CLIENTFadeOutLobby _aslobby_player_controller_bp))
  (Utilities|FlowControl|Delay 1.5)
  (Class|TestingGamemode|LoadIntoActualGame))

(event EventFadeOutIntoGame
  (bind _astesting_game_state (Utilities|Casting|CastToTestingGameState (Game|GetGameState)))
  (bind _returnvalue (Class|TestingGameState|GetPlayersConnected _astesting_game_state))
  (for _array_element _returnvalue
    (bind _aslobby_player_controller_bp (Utilities|Casting|CastToLobbyPlayerController_BP _array_element))
    (Default|CLIENTRemoveLobbyUI _aslobby_player_controller_bp)))

(fn ConstructionScript)